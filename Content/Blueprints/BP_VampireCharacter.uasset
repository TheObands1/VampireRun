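; BP_VampireCharacter is a character Blueprint that handles top-level movement and HUD setup for a vampire character.
; On BeginPlay it creates the WB_HUD widget and adds it to the viewport.
; Each tick it normalizes the forward and right inputs into a world-space direction, snaps the actor's rotation to face it and adds movement input along it.
; Taking damage only prints a debug string.
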(event `self.ReceiveBeginPlay`
  (bind _returnvalue (`|CreateWidget` "/Game/UI/HUD/WB_HUD.WB_HUD_C"))
  (`UserWidget.AddToViewport` _returnvalue 0))

(event `self.ReceiveTick`
  (params (DeltaSeconds :type "Float (single-precision)"))
  (bind _output_get (set `self.BP_MoveDirection` (`KismetMathLibrary.Normal` (`KismetMathLibrary.MakeVector` (`self.GetInputAxisValue`) (`self.GetInputAxisValue`)))))
  (if (> (`KismetMathLibrary.VSize` _output_get) 0.0)
    (`self.K2_SetActorRotation` (`KismetMathLibrary.MakeRotFromX` (`self.BP_MoveDirection`)))
    (`self.AddMovementInput` (`self.BP_MoveDirection`))))

(event `self.ReceiveAnyDamage`
  (params (Damage :type "Float (single-precision)") (DamageType :type "DamageType Object Reference") (InstigatedBy :type "Controller Object Reference") (DamageCauser :type "Actor Object Reference"))
  (`KismetSystemLibrary.PrintString` "Hello" true true (struct :`G` 0.66 :`B` 1.0 :`A` 1.0) 1.0))

(fn `UserConstructionScript`)